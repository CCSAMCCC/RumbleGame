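; Storage room door actor that opens once both the hour and minute conditions of a puzzle are correct.
; External events set or clear each flag, and each "correct" event rechecks both through Open.
; When both are true, Open plays 2D door and creak sounds, then a timeline lerps the actor's absolute rotation to a 90-degree swing.
; Open has no already-opened guard, so a repeated correct event replays the sounds and animation.
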(event `MinuteFalse`
  (set `self.MinCor` false))

(event `HourFalse`
  (set `self.HourCor` false))

(event `MinuteCorrect`
  (set `self.MinCor` true)
  (`self.Open`))

(event `HourCorrect`
  (set `self.HourCor` true)
  (`self.Open`))

(event `Open`
  (if (and (`self.HourCor`) (`self.MinCor`))
    (`GameplayStatics.PlaySound2D` "/Game/SamStuff/Thomas/C_DoorOpen.C_DoorOpen" 1.0 1.0 0.0 null null)
    (`GameplayStatics.PlaySound2D` "/Game/SamStuff/Thomas/C_Creak.C_Creak" 1.0 1.0 0.0 null null)
    (bind (_direction _newtrack_0) (`Timeline|Timeline` :!via `PlayFromStart`)
      (:`Update`
        (`self.K2_SetActorRotation` (`KismetMathLibrary.RLerp` (struct) (struct :`Yaw` 90.0) _newtrack_0))))))

(fn `UserConstructionScript`)