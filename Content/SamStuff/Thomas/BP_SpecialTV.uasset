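; BP_SpecialTV is a television that cycles through channel screens and plays a static sound at its location on BeginPlay.
; While Active, SwitchChannels loops by calling itself, using delayed material swaps from static through solid-color screens to black.
; Settle shows the TVTIME material and clears Active.
; A cycle already running keeps swapping until its next Active check, which then restores TVTIME.
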(event `self.ReceiveBeginPlay`
  (`self.SwitchChannels`)
  (`GameplayStatics.PlaySoundAtLocation` "/Game/SamStuff/Thomas/C_Static.C_Static" (`SceneComponent.K2_GetComponentLocation` (`self.DefaultSceneRoot`)) (struct) 1.0 1.0 0.0 "/Game/SamStuff/Thomas/NewSoundAttenuation.NewSoundAttenuation" null null null))

(event `SwitchChannels`
  (bind _tv (`self.TV`))
  (if (`self.Active`)
    (`PrimitiveComponent.SetMaterial` _tv 0 "/Game/SamStuff/ConferenceRoom/Materials/MI/MI_TVSTATIC.MI_TVSTATIC")
    (`KismetSystemLibrary.Delay` 3.0)
    (`PrimitiveComponent.SetMaterial` _tv 0 "/Game/SamStuff/ConferenceRoom/Materials/MI/MI_TVRED.MI_TVRED")
    (`KismetSystemLibrary.Delay` 0.5)
    (`PrimitiveComponent.SetMaterial` _tv 0 "/Game/SamStuff/ConferenceRoom/Materials/MI/MI_TVGREEN.MI_TVGREEN")
    (`KismetSystemLibrary.Delay` 0.5)
    (`PrimitiveComponent.SetMaterial` _tv 0 "/Game/SamStuff/ConferenceRoom/Materials/MI/MI_TVBLUE.MI_TVBLUE")
    (`KismetSystemLibrary.Delay` 0.5)
    (`PrimitiveComponent.SetMaterial` _tv 0 "/Game/SamStuff/ConferenceRoom/Materials/MI/MI_TVYELLOW.MI_TVYELLOW")
    (`KismetSystemLibrary.Delay` 0.5)
    (`PrimitiveComponent.SetMaterial` _tv 0 "/Game/SamStuff/ConferenceRoom/Materials/MI/MI_TVBLACK.MI_TVBLACK")
    (`KismetSystemLibrary.Delay` 0.5)
    (`self.SwitchChannels`)
    (else
      (`PrimitiveComponent.SetMaterial` (`self.TV`) 0 "/Game/SamStuff/ConferenceRoom/Materials/MI/MI_TVTIME.MI_TVTIME" :!label _label)
      (set `self.Active` false))))

(event `Settle`
  (goto _label))

(fn `UserConstructionScript`)