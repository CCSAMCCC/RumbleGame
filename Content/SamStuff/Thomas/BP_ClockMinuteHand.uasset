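; BP_ClockMinuteHand is a clickable clock minute hand for a puzzle tied to BP_StorageRoomDoor.
; Hovering swaps the plane's material, and each click plays a tick and runs a timeline that rotates the actor one fixed step.
; The tracked angle wraps after a full turn, then the door is told whether the hand is at the correct position.
; A DoOnce blocks further clicks until each step finishes.
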(event `self.Plane.OnBeginCursorOver`
  (params (TouchedComponent :type "PrimitiveComponent Object Reference"))
  (`PrimitiveComponent.SetMaterial` (`self.Plane`) 0 "/Game/SamStuff/Thomas/M_MinHandHov.M_MinHandHov"))

(event `self.Plane.OnEndCursorOver`
  (params (TouchedComponent :type "PrimitiveComponent Object Reference"))
  (`PrimitiveComponent.SetMaterial` (`self.Plane`) 0 "/Game/SamStuff/Thomas/M_MinHand.M_MinHand"))

(event `self.Plane.OnClicked`
  (params (TouchedComponent :type "PrimitiveComponent Object Reference") (ButtonPressed :type "Key Structure"))
  (bind _currentrot (`self.CurrentRot`))
  (bind _returnvalue (+ _currentrot 18.0))
  (`/Engine/EditorBlueprintResources/StandardMacros.DoOnce` false :!label _label
    (:`Completed`
      (`GameplayStatics.PlaySound2D` "/Game/SamStuff/Thomas/C_Tic.C_Tic" 1.0 1.0 0.0 null null)
      (bind (_direction _newtrack_0) (`Timeline|adjust` :!via `PlayFromStart`)
        (:`Update`
          (`self.K2_SetActorRotation` (`KismetMathLibrary.MakeRotator` 90.0 (`KismetMathLibrary.Lerp` _currentrot _returnvalue _newtrack_0))))
        (:`Finished`
          (if (>= _currentrot 342.0)
            (set `self.CurrentRot` 0.0)
            (else
              (bind _output_get (set `self.CurrentRot` _returnvalue))))
          (if (== _output_get 90.0)
            (`KismetSystemLibrary.PrintString` "Minute Hand Correct")
            (bind _returnvalue_2 (`GameplayStatics.GetActorOfClass` "/Game/SamStuff/Thomas/BP_StorageRoomDoor.BP_StorageRoomDoor_C"))
            (`/Game/SamStuff/Thomas/BP_StorageRoomDoor.MinuteCorrect` _returnvalue_2)
            (goto _label :!via `Reset`)
            (else
              (bind _returnvalue_3 (`GameplayStatics.GetActorOfClass` "/Game/SamStuff/Thomas/BP_StorageRoomDoor.BP_StorageRoomDoor_C"))
              (`/Game/SamStuff/Thomas/BP_StorageRoomDoor.MinuteFalse` _returnvalue_3)
              (goto _label :!via `Reset`))))))))

(fn `UserConstructionScript`)