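; BP_TestObject is a test actor for a clickable item that can be inspected in a close-up UI.
; Cursor hover events swap the cube's material.
; A click plays a timeline that shrinks the cube to zero scale, then after a short delay creates a W_ItemCloseup widget filled with the item's image, text and a self reference.
; The PutDown event reverses the timeline from the end.
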(event `self.Cube.OnBeginCursorOver`
  (params (TouchedComponent :type "PrimitiveComponent Object Reference"))
  (`PrimitiveComponent.SetMaterial` (`self.Cube`) 0 "/Game/SamStuff/BroadcastStudio/Materials/Instances/MI_BS_TrimTexture_02.MI_BS_TrimTexture_02"))

(event `self.Cube.OnEndCursorOver`
  (params (TouchedComponent :type "PrimitiveComponent Object Reference"))
  (`PrimitiveComponent.SetMaterial` (`self.Cube`) 0 "/Game/SamStuff/BroadcastStudio/Materials/Instances/MI_FlowerPlant.MI_FlowerPlant"))

(event `self.Cube.OnClicked`
  (params (TouchedComponent :type "PrimitiveComponent Object Reference") (ButtonPressed :type "Key Structure"))
  (`|ExecutionSequence`
    (:`then_0`
      (bind (_direction _newtrack_0) (`Timeline|Clicked` :!label _label)
        (:`Update`
          (`SceneComponent.SetRelativeScale3D` (`self.Cube`) (`KismetMathLibrary.VLerp` (0.5 0.5 0.5) (0.0 0.0 0.0) _newtrack_0)))))
    (:`then_1`
      (`KismetSystemLibrary.Delay` 0.75)
      (bind _returnvalue (`|CreateWidget` "/Game/SamStuff/Thomas/W_ItemCloseup.W_ItemCloseup_C" (`GameplayStatics.GetPlayerController` 0)))
      (`UserWidget.AddToViewport` _returnvalue 0)
      (`/Game/SamStuff/Thomas/W_ItemCloseup.FillInfo` _returnvalue (`self.2dimage`) (`self.Text`) self))))

(event `PutDown`
  (goto _label :!via `ReverseFromEnd`))

(fn `UserConstructionScript`)