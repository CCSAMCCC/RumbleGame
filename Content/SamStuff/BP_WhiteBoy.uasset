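; BP_WhiteBoy is an AI-controlled actor that wanders around the point where it starts play.
; BeginPlay stores that location and, after the minimum roam interval, starts the movement loop.
; Each cycle uses AI Move To toward a random reachable point within roam range of the stored location.
; Whether the move finishes or fails, it waits a random time between the interval limits and picks again.
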(event `self.ReceiveBeginPlay`
  (set `self.Spawn Location` (`self.K2_GetActorLocation`))
  (`KismetSystemLibrary.Delay` (`self.Roam Interval Min`))
  (`self.Go to random location`))

(event `Go to random location`
  (`AITask_MoveTo.AIMoveTo` (`AIBlueprintHelperLibrary.GetAIController` self) (`NavigationSystemV1.K2_GetRandomReachablePointInRadius` (`self.Spawn Location`) (`self.RoamRange`) null null) null
    (:`OnRequestFailed`
      _)
    (:`OnMoveFinished`
      _))
  (`KismetSystemLibrary.Delay` (`KismetMathLibrary.RandomFloatInRange` (`self.Roam Interval Min`) (`self.Roam Interval Max`)))
  (`self.Go to random location`))

(fn `UserConstructionScript`)