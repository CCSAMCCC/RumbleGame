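; BP_TransCielingCrypt is a crypt actor that changes its roof materials around the player, apparently to make the ceiling see-through.
; When a BP_ThirdPersonCharacter enters its Box trigger, the Crypt component's shingle and wood beam slots switch to alternate material instances, presumably transparent variants.
; Leaving the box restores the standard materials; the swap is immediate, with no fade or Tick logic.
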(event `self.Box.OnComponentBeginOverlap`
  (params (OverlappedComponent :type "PrimitiveComponent Object Reference") (OtherActor :type "Actor Object Reference") (OtherComp :type "PrimitiveComponent Object Reference") (OtherBodyIndex :type Integer) (bFromSweep :type Boolean) (SweepResult :type "HitResult Structure (by ref)"))
  (cast `/Game/ThirdPerson/Blueprints/BP_ThirdPersonCharacter` OtherActor)
  (`PrimitiveComponent.SetMaterial` (`self.Crypt`) 5 "/Game/Necropolis/Materials/MI_shingles1.MI_shingles1")
  (`PrimitiveComponent.SetMaterial` (`self.Crypt`) 3 "/Game/Necropolis/Materials/MI_wood_beams1.MI_wood_beams1"))

(event `self.Box.OnComponentEndOverlap`
  (params (OverlappedComponent :type "PrimitiveComponent Object Reference") (OtherActor :type "Actor Object Reference") (OtherComp :type "PrimitiveComponent Object Reference") (OtherBodyIndex :type Integer))
  (cast `/Game/ThirdPerson/Blueprints/BP_ThirdPersonCharacter` OtherActor)
  (`PrimitiveComponent.SetMaterial` (`self.Crypt`) 5 "/Game/Necropolis/Materials/MI_shingles.MI_shingles")
  (`PrimitiveComponent.SetMaterial` (`self.Crypt`) 3 "/Game/Necropolis/Materials/MI_wood_beams.MI_wood_beams"))

(fn `UserConstructionScript`)